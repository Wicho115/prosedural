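; BP_Room2 is a procedural generator room Blueprint that holds a collectible pickup for the player.
; When BP_ThirdPersonCharacter overlaps Sphere1, it destroys the separate Sphere component and increments the Recolectados (collected) counter on BP_ThirdPersonGameMode.
; Debug prints show the player detection and the new count.
; Sphere1 itself is not destroyed or disabled here, so repeat overlaps can raise the count again.
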(event `self.Sphere1.OnComponentBeginOverlap`
  (params (OverlappedComponent :type "PrimitiveComponent Object Reference") (OtherActor :type "Actor Object Reference") (OtherComp :type "PrimitiveComponent Object Reference") (OtherBodyIndex :type Integer) (bFromSweep :type Boolean) (SweepResult :type "HitResult Structure (by ref)"))
  (cast `/Game/ThirdPerson/Blueprints/BP_ThirdPersonCharacter` OtherActor)
  (`KismetSystemLibrary.PrintString` "Es jugador")
  (`ActorComponent.K2_DestroyComponent` (`self.Sphere`))
  (bind _asbp_third_person_game_mode (cast `/Game/ThirdPerson/Blueprints/BP_ThirdPersonGameMode` (`GameplayStatics.GetGameMode`)))
  (bind _output_get (set `/Game/ThirdPerson/Blueprints/BP_ThirdPersonGameMode.Recolectados` (+ (`/Game/ThirdPerson/Blueprints/BP_ThirdPersonGameMode.Recolectados` _asbp_third_person_game_mode) 1) _asbp_third_person_game_mode))
  (`KismetSystemLibrary.PrintString` (`KismetStringLibrary.Conv_IntToString` _output_get)))

(fn `UserConstructionScript`
  (`parent.UserConstructionScript`))