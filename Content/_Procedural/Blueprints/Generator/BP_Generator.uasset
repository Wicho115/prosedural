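; BP_Generator is a procedural generator actor that builds a grid of room prefabs from a JSON map when play begins.
; It reads the matrix, row count and column count from MapJSON.
; Each non-zero cell spawns the matching PrefabRoooms class, indexed by value minus one, offset from the generator's location.
; The flat array index becomes column and row via Columns, scaled by XValue along X and ZValue along Y.
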(event `self.ReceiveBeginPlay`
  (bind _columns (`self.columns`))
  (bind _outjsonobject (`JsonBlueprintFunctionLibrary.FromFile` (`self.mapJSON`)))
  (`|ExecutionSequence`
    (:`then_0`
      (bind _outvalue (`|GetJsonField` _outjsonobject "matrix"))
      (set `self.matrix` _outvalue))
    (:`then_1`
      (bind _outvalue_2 (`|GetJsonField` _outjsonobject "rows"))
      (set `self.rows` _outvalue_2))
    (:`then_2`
      (bind _outvalue_3 (`|GetJsonField` _outjsonobject "columns"))
      (set `self.columns` _outvalue_3))
    (:`then_3`
      ;[1 1 1] Creacion de rooms
      (for (_array_element _array_index) (`self.matrix`)
        (if (!= _array_element 0)
          (bind _returnvalue (/ _array_index _columns))
          (`|SpawnActorFromClass` (`|GetArrayItem` (`self.PrefabRoooms`) (- _array_element 1)) (`KismetMathLibrary.MakeTransform` (+ (`self.K2_GetActorLocation`) (`KismetMathLibrary.MakeVector` (`KismetMathLibrary.Conv_IntToDouble` (* (- _array_index (* _returnvalue _columns)) (`self.xValue`))) (`KismetMathLibrary.Conv_IntToDouble` (* _returnvalue (`self.zValue`))) 0.0))) "Undefined" "MultiplyWithRoot" null null))))))

(fn `UserConstructionScript`)